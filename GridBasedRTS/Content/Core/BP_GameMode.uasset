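; Game mode that sets up a debug UI and cursor input for a hex grid game.
; On BeginPlay it adds the W_DebugMenu widget, sets permanent mouse capture, shows the cursor and caches the level's BP_HexGrid, which is not used afterward.
; Every Tick it runs a complex trace under the cursor and prints whether it hit, as a debug readout.
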(event `self.ReceiveBeginPlay`
  (bind _returnvalue (`|CreateWidget` "/Game/Core/Debug/W_DebugMenu.W_DebugMenu_C"))
  (bind _output_get (set `self.DebugMenu` _returnvalue))
  (`UserWidget.AddToViewport` _output_get 0)
  (`GameplayStatics.SetViewportMouseCaptureMode` "CapturePermanently")
  (bind _output_get_2 (set `self.PlayerController` (`GameplayStatics.GetPlayerController` 0)))
  (set `PlayerController.bShowMouseCursor` true _output_get_2)
  (bind _returnvalue_2 (`GameplayStatics.GetActorOfClass` "/Game/Core/BP_HexGrid.BP_HexGrid_C"))
  (set `self.Grid` _returnvalue_2))

(event `self.ReceiveTick`
  (params (DeltaSeconds :type "Float (single-precision)"))
  (`KismetSystemLibrary.PrintString` (`KismetStringLibrary.Conv_BoolToString` (`GameplayStatics.BreakHitResult` (`PlayerController.GetHitResultUnderCursorByChannel` (`self.PlayerController`) "TraceTypeQuery3" true)))))

(fn `UserConstructionScript`)